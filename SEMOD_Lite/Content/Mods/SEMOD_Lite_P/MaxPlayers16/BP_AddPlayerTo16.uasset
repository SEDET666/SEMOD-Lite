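; Server-side mod actor that expands player list UI for up to 16 players, destroying itself on clients, menu/splash maps or game versions below 1.3.
; A one-second timer resizes lobby list widgets to the game instance's MaxPlayers and rebinds entries by player controller index.
; In Lobby it copies MaxPlayers to the game state.
; Elsewhere it appends fixed extra VOIP entries, updating them on a second timer.
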(event Custom|RefreshPlayerList
  (params (ScrollBox :type Panel%20Widget%20Object%20Reference))
  ;[1 1 1] 手动刷新玩家列表代码
  (for (_array_element _array_index) (Class|PanelWidget|GetAllChildren ScrollBox)
    (if (== (Utilities|GetClass _array_element) "/Game/UI/Lobby/PlayerList/W_Lobby_PlayerList_Entry.W_Lobby_PlayerList_Entry_C")
      (bind _asw_lobby_player_list_entry (Utilities|Casting|CastToW_Lobby_PlayerList_Entry _array_element)
        (:then
          _)
        (:CastFailed
          _))
      (bind _outactors (Actor|GetAllActorsOfClass "/Script/Engine.PlayerController"))
      (if (< _array_index (Utilities|Array|Length _outactors))
        (Default|SetPlayer _asw_lobby_player_list_entry (Class|AdvancedSessionsLibrary|GetUniqueNetID (Game|GetPlayerController _array_index)))
        (else
          (Default|ClearPlayer _asw_lobby_player_list_entry))))))

(event Custom|刷新
  ;[1 1 1] 手动刷新玩家列表代码
  (bind _foundwidgets (Widget|GetAllWidgetsOfClass "/Game/UI/Lobby/PlayerList/W_Lobby_PlayerList.W_Lobby_PlayerList_C" false))
  (for _array_element _foundwidgets
    (CallFunction|RefreshPlayerList (Widget|GetParent (Variables|/Game/UI/Lobby/PlayerList/W_Lobby_PlayerList.W_Lobby_PlayerList_C|GetEntry0 _array_element)))))

(event Custom|初始化VOIPPLAYERLIST
  (bind _foundwidgets (Widget|GetAllWidgetsOfClass "/Game/UI/Online/W_VOIP_PlayerList.W_VOIP_PlayerList_C" true))
  (for _array_element _foundwidgets
    (for _index (range 5 16)
      (bind _returnvalue (UserInterface|CreateWidget "/Game/UI/Online/W_VOIP_PlayerList_Entry.W_VOIP_PlayerList_Entry_C" (Game|GetPlayerController 0)))
      (Widget|Panel|AddChild (Widget|GetParent (Variables|/Game/UI/Online/W_VOIP_PlayerList.W_VOIP_PlayerList_C|GetW_VOIP_PlayerList_Entry1 _array_element)) _returnvalue)))
  (CallFunction|更新voipentry))

(event Custom|初始化
  (bind _maxplayer (CallFunction|GetMaxPlayers))
  (bind _entrys (Variables|Default|GetEntrys))
  (bind _returnvalue (Utilities|Array|Length _entrys))
  (bind _returnvalue_2 (- _returnvalue 1))
  (bind _foundwidgets (Widget|GetAllWidgetsOfClass "/Game/UI/Lobby/PlayerList/W_Lobby_PlayerList.W_Lobby_PlayerList_C" false))
  (for _array_element _foundwidgets
    (Variables|Default|SetC 0)
    (Utilities|Array|Clear (Variables|Default|GetEntrys))
    (for _array_element_2 (Class|PanelWidget|GetAllChildren (Widget|GetParent (Variables|/Game/UI/Lobby/PlayerList/W_Lobby_PlayerList.W_Lobby_PlayerList_C|GetEntry0 _array_element)))
      (if (== (Utilities|GetClass _array_element_2) "/Game/UI/Lobby/PlayerList/W_Lobby_PlayerList_Entry.W_Lobby_PlayerList_Entry_C")
        (bind _asw_lobby_player_list_entry (Utilities|Casting|CastToW_Lobby_PlayerList_Entry _array_element_2)
          (:then
            _)
          (:CastFailed
            _))
        (Variables|Default|SetC (+ (Variables|Default|GetC) 1))
        (Utilities|Array|Add (Variables|Default|GetEntrys) _asw_lobby_player_list_entry)))
    (if (< (Variables|Default|GetC) _maxplayer)
      (for _index (range 1 (- _maxplayer (Variables|Default|GetC)))
        (bind _returnvalue_3 (UserInterface|CreateWidget "/Game/UI/Lobby/PlayerList/W_Lobby_PlayerList_Entry.W_Lobby_PlayerList_Entry_C" (Game|GetPlayerController 0)))
        (Widget|Panel|AddChild (Widget|GetParent (Variables|/Game/UI/Lobby/PlayerList/W_Lobby_PlayerList.W_Lobby_PlayerList_C|GetEntry0 _array_element)) _returnvalue_3))
      (Variables|/Game/UI/Lobby/PlayerList/W_Lobby_PlayerList.W_Lobby_PlayerList_C|SetPlayerListEntries _array_element (Variables|Default|GetEntrys))
      (elif (> (Variables|Default|GetC) _maxplayer)
        (for _index_2 (range 1 (- (Variables|Default|GetC) _maxplayer))
          (Widget|RemovefromParent (Utilities|Array|Get(acopy) _entrys _returnvalue_2))
          (Utilities|Array|RemoveIndex _entrys _returnvalue_2))
        (Variables|/Game/UI/Lobby/PlayerList/W_Lobby_PlayerList.W_Lobby_PlayerList_C|SetPlayerListEntries _array_element (Variables|Default|GetEntrys)))))
  (CallFunction|刷新))

(event Custom|更新voipentry
  (bind _foundwidgets (Widget|GetAllWidgetsOfClass "/Game/UI/Online/W_VOIP_PlayerList.W_VOIP_PlayerList_C" true))
  (for _array_element _foundwidgets
    (for _index (range 4 15)
      (bind _asw_voip_player_list_entry (Utilities|Casting|CastToW_VOIP_PlayerList_Entry (Utilities|Array|Get(acopy) (Class|PanelWidget|GetAllChildren (Widget|GetParent (Variables|/Game/UI/Online/W_VOIP_PlayerList.W_VOIP_PlayerList_C|GetW_VOIP_PlayerList_Entry1 _array_element))) _index))
        (:then
          _)
        (:CastFailed
          _))
      (bind _outactors (Actor|GetAllActorsOfClass "/Script/Engine.PlayerController"))
      (if (< _index (Utilities|Array|Length _outactors))
        (Widget|SetVisibility _asw_voip_player_list_entry "Visible")
        (Default|SetPlayer _asw_voip_player_list_entry (Class|AdvancedSessionsLibrary|GetUniqueNetID (Game|GetPlayerController _index)))
        (else
          (Widget|SetVisibility _asw_voip_player_list_entry "Hidden"))))))

(event EventEndPlay
  (params (EndPlayReason :type EEndPlayReason%20Enum :default "Destroyed"))
  (Utilities|Time|ClearandInvalidateTimerbyHandle (stale EventBeginPlay _returnvalue_3))
  (Utilities|Time|ClearandInvalidateTimerbyHandle (stale EventBeginPlay _returnvalue_5)))

(event EventBeginPlay
  (bind _returnvalue (Game|GetCurrentLevelName true))
  (if (Utilities|Enum|Equal(Enum) _returnvalue "MainMenuMap")
    (Actor|DestroyActor :!label _label)
    (elif (Utilities|Enum|Equal(Enum) _returnvalue "SplashScreenMap")
      (goto _label)
      (elif (Networking|IsServer)
        (bind _returnvalue_2 (Class|FancyPlatformUtilsLibrary|GetGameVersion))
        (if (>= (Math|Conversions|ToFloat(Integer) (Utilities|String|Left _returnvalue_2 3)) 1.3)
          (CallFunction|初始化)
          (bind _returnvalue_3 (Utilities|Time|SetTimerbyEvent (delegate Custom|初始化) 1.0 true))
          (if (Networking|IsServer)
            (Utilities|FlowControl|Delay 1.0)
            (if (Utilities|Enum|Equal(Enum) _returnvalue "Lobby")
              (bind _returnvalue_4 (Actor|GetActorOfClass "/Game/Multiplayer/Lobby_GS.Lobby_GS_C"))
              (Variables|/Game/Multiplayer/Lobby_GS.Lobby_GS_C|SetMaxPlayers _returnvalue_4 (CallFunction|GetMaxPlayers))
              (else
                (CallFunction|初始化VOIPPLAYERLIST)
                (bind _returnvalue_5 (Utilities|Time|SetTimerbyEvent (delegate Custom|更新voipentry) 1.0 true)))))
          (else
            (goto _label)))
        (else
          (goto _label))))))

(fn ConstructionScript)

(fn GetMaxPlayers
  (bind _asbp_my_game_instance (Utilities|Casting|CastToBP_MyGameInstance (Game|GetGameInstance))
    (:then
      _)
    (:CastFailed
      _))
  (return (Variables|/Game/MainMenu/Blueprints/BP_MyGameInstance.BP_MyGameInstance_C|GetMaxPlayers _asbp_my_game_instance)))