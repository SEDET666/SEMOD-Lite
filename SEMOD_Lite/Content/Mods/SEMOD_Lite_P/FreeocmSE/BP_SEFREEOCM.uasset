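; BP_SEFREEOCM is a mod actor that lets the player use an InteractableActor under the screen center with the F key.
; It disables its own collision on BeginPlay and polls the first player controller for the key every Tick.
; A helper line-traces on Visibility from the camera along the deprojected viewport center and returns the hit actor and distance.
; Close hits of that class receive OnActorUsedMessage with the player character.
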(event EventTick
  (params (DeltaSeconds :type Float%20%28single-precision%29))
  (if (Game|Player|WasInputKeyJustPressed (Game|GetPlayerController 0) "F")
    (bind (_actor _距离) (CallFunction|射线检测Interact))
    (if (Utilities|ClassIsChildOf (Utilities|GetClass _actor) "/Script/Backrooms.InteractableActor")
      (if (< _距离 2e+02)
        (bind _asinteractable_actor (Utilities|Casting|CastToInteractableActor _actor))
        (Class|InteractableInterface|OnActorUsed(Message) _asinteractable_actor (Game|GetPlayerCharacter 0))))))

(event EventBeginPlay
  (Collision|SetActorEnableCollision false))

(fn ConstructionScript)

(fn 射线检测Interact
  (params (玩家ID :type Integer))
  (bind _returnvalue (Viewport|GetViewportSize))
  (bind _returnvalue_2 (Game|GetPlayerCameraManager 玩家ID))
  (bind _returnvalue_3 (* _returnvalue 0.5))
  (bind _returnvalue_4 (Camera|GetCameraLocation _returnvalue_2))
  (bind _outhit (Collision|LineTraceByChannel _returnvalue_4 (+ _returnvalue_4 (* (.WorldDirection (Class|PlayerController|DeprojectScreenPositiontoWorld (Game|GetPlayerController 玩家ID) (.x _returnvalue_3) (.y _returnvalue_3))) 1e+04)) "TraceTypeQuery1" false 0 "None"))
  (return (.HitActor (Collision|BreakHitResult _outhit)) (.Distance (Collision|BreakHitResult _outhit))))