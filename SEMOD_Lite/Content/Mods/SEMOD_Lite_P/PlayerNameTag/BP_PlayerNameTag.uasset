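; BP_PlayerNameTag is a floating name tag actor that shows a player's name above their pawn.
; On BeginPlay it caches the WBP_PlayerNameTag from its Widget component.
; Each tick it teleports above the pawn at player index ID, sets its yaw opposite player 0's pawn rotation, and writes that player's PlayerState name into the widget.
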(event EventBeginPlay
  (bind _aswbp_player_name_tag (Utilities|Casting|CastToWBP_PlayerNameTag (UserInterface|GetWidget (Variables|Default|GetWidget))))
  (Variables|Default|SetNameWidget _aswbp_player_name_tag))

(event EventTick
  (params (DeltaSeconds :type Float%20%28single-precision%29))
  (bind _id (Variables|Default|GetID))
  (bind _returnvalue (Game|Player|GetPlayerPawn _id))
  (bind _returnvalue_2 (Transformation|GetActorLocation _returnvalue))
  (Transformation|SetActorLocationAndRotation (Math|Vector|MakeVector (.x _returnvalue_2) (.y _returnvalue_2) (+ (.z _returnvalue_2) 1.2e+02)) (Math|Rotator|MakeRotator 0.0 0.0 (- (.yaw (Transformation|GetActorRotation (Game|Player|GetPlayerPawn 0))) 1.8e+02)) false true)
  (Variables|/Game/Mods/SEMOD_Lite_P/PlayerNameTag/WBP_PlayerNameTag.WBP_PlayerNameTag_C|Setplayernameshow (Variables|Default|GetNameWidget) (PlayerState|GetPlayerName (Variables|/Script/Engine.Pawn|GetPlayerState _returnvalue))))

(fn ConstructionScript)